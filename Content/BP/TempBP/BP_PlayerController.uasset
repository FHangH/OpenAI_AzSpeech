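; Player controller that toggles an achievement list UI and switches between game and UI input for BP_Player.
; Tab shows or hides the list through the BPCompAS component once it has loaded, then calls ChangeControllerInputMode.
; That event uses the ChangeInputMode macro to set input mode and cursor visibility, and disables character movement in UI mode.
; Keys 1–3 each trigger a one-shot achievement task on the component.
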(event Custom|ChangeControllerInputMode
  (params (IsGameInput :type Boolean))
  (Utilities|ChangeInputMode IsGameInput
    (:GameMode
      (Variables|Default|SetbShowMouseCursor false)
      (bind _asbp_player (Utilities|Casting|CastToBP_Player (Pawn|GetControlledPawn)))
      (Components|Activation|SetActive (Variables|/Script/Engine.Character|GetCharacterMovement _asbp_player) true false))
    (:UIMode
      (Variables|Default|SetbShowMouseCursor true)
      (bind _asbp_player_2 (Utilities|Casting|CastToBP_Player (Pawn|GetControlledPawn)))
      (Components|Activation|SetActive (Variables|/Script/Engine.Character|GetCharacterMovement _asbp_player_2) false false))))

(event Input|KeyboardEvents|1
  (params (Key :type Key%20Structure :default "None"))
  (:Pressed
    (Default|DoOnceTaskAchievements (Variables|Default|GetBP_Comp_AS))))

(event Input|KeyboardEvents|2
  (params (Key :type Key%20Structure :default "None"))
  (:Pressed
    (Default|DoOnceTaskAchievements (Variables|Default|GetBP_Comp_AS) 1)))

(event Input|KeyboardEvents|3
  (params (Key :type Key%20Structure :default "None"))
  (:Pressed
    (Default|DoOnceTaskAchievements (Variables|Default|GetBP_Comp_AS) 2)))

(event Input|KeyboardEvents|Tab
  (params (Key :type Key%20Structure :default "None"))
  (:Pressed
    (if (Variables|/Game/BP/AS/BP_Comp_AS.BP_Comp_AS_C|GetIsAListLoadOver (Variables|Default|GetBP_Comp_AS))
      (if (Variables|Default|GetIsShow)
        (Default|HideUIAList (Variables|Default|GetBP_Comp_AS))
        (Variables|Default|SetIsShow false)
        (CallFunction|ChangeControllerInputMode true)
        (else
          (Default|ShowUIAList (Variables|Default|GetBP_Comp_AS))
          (Variables|Default|SetIsShow true)
          (CallFunction|ChangeControllerInputMode false))))))

(fn ConstructionScript)