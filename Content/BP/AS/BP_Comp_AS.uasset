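; Achievement system component that registers sample key-press achievements and drives their list UI.
; On BeginPlay it creates the list widget, then clears and rebuilds the achievement list, mostly cumulative entries with grades and images, and fills the widget.
; DoOnceTask_Achievements advances an achievement by ID, refreshes its UI entry and shows a tip once it completes.
; Other events show or hide the list and update single items, matched by their displayed ID text.
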(event Custom|UpdateUI_AItem
  (params (AchievementID :type Integer))
  (bind _returnvalue (Class|FHFuncLibAS|GetAchievementsList))
  (bind _ui_alist (Variables|Default|GetUI_Alist))
  (bind (_value _returnvalue_2) (Utilities|Map|Find _returnvalue AchievementID))
  (bind _scrollbox_a (Variables|/Game/BP/AS/UI_ASList.UI_ASList_C|GetScrollBox_A _ui_alist))
  (Utilities|IsValid _scrollbox_a
    (:Is%20Valid
      (for _array_element (Class|PanelWidget|GetAllChildren _scrollbox_a)
        (bind _asui_aitem (Utilities|Casting|CastToUI_AItem _array_element))
        (if (Utilities|Enum|Equal(Enum) (Variables|/Script/UMG.TextBlock|GetText (Variables|/Game/BP/AS/UI_AItem.UI_AItem_C|GetTextBlock_AID _asui_aitem)) (Utilities|Text|FormatText "ID:{id}" AchievementID))
          (if _returnvalue_2
            (Default|SetUIAchievementItem _asui_aitem _value)))))))

(event Custom|DoOnceTask_Achievements
  (params (AchievementID :type Integer))
  (bind (_id _isdoover) (Class|FHFuncLibAS|DoOnceTask AchievementID))
  (if _isdoover
    (CallFunction|UpdateUIAItem _id)
    (if (Class|FHFuncLibAS|IsAchievementComplete _id)
      (Default|ShowTip (Variables|Default|GetUI_Alist) _id))))

(event Custom|ShowUI_AList
  (Utilities|IsValid (Variables|Default|GetUI_Alist)
    (:Is%20Valid
      (bind _achievements (Class|FHFuncLibAS|GetAllAchievements))
      (Default|ShowAchievementsList (Variables|Default|GetUI_Alist) _achievements))))

(event Custom|HideUI_AList
  (Utilities|IsValid (Variables|Default|GetUI_Alist)
    (:Is%20Valid
      (Default|HideAchievementsList (Variables|Default|GetUI_Alist)))))

(event EventBeginPlay
  (Utilities|FlowControl|Sequence
    (:then_0
      (Utilities|InitAListUI))
    (:then_1
      (Utilities|InitAchievementSystem)
      (bind _achievements (Class|FHFuncLibAS|GetAllAchievements))
      (Default|UpdateAchievementsList (Variables|Default|GetUI_Alist) _achievements))))