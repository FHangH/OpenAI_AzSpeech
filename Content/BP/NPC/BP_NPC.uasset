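; BP_NPC is a talking NPC that voice-chats through a GPT component (BPCompGPT) when a tagged actor enters its sphere.
; Overlap toggles AudioCapture and the chat widget; activation sends a default greeting, and envelope volume above a threshold triggers voice recording.
; GPT callbacks update the chat and network-status UIs.
; Without network, it plays local introduction or warning sounds, while deactivation clears the GPT task.
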(event OnComponentBeginOverlap(Sphere)
  (params (OverlappedComponent :type Primitive%20Component%20Object%20Reference) (OtherActor :type Actor%20Object%20Reference) (OtherComp :type Primitive%20Component%20Object%20Reference) (OtherBodyIndex :type Integer) (bFromSweep :type Boolean) (SweepResult :type Hit%20Result%20Structure%20%28by%20ref%29))
  (Utilities|IsValid OtherActor
    (:Is%20Valid
      (if (Actor|ActorHasTag OtherActor (Variables|OpenAI|GetChatTag))
        (Components|Activation|SetActive (Variables|Default|GetAudioCapture) true false)
        (if (Default|CheckNetworking (Variables|Default|GetBP_Comp_GPT)) ; 网络判断，成功创建文本UI，失败隐藏UI
          (Rendering|SetVisibility (Variables|Default|GetWidget) true false)
          (else
            (Rendering|SetVisibility (Variables|Default|GetWidget) false false)))))))

(event OnComponentEndOverlap(Sphere)
  (params (OverlappedComponent :type Primitive%20Component%20Object%20Reference) (OtherActor :type Actor%20Object%20Reference) (OtherComp :type Primitive%20Component%20Object%20Reference) (OtherBodyIndex :type Integer))
  (Utilities|IsValid OtherActor
    (:Is%20Valid
      (if (Actor|ActorHasTag OtherActor (Variables|OpenAI|GetChatTag))
        (Components|Activation|SetActive (Variables|Default|GetAudioCapture) false false)
        (Rendering|SetVisibility (Variables|Default|GetWidget) false false)))))

(event OnComponentActivated(AudioCapture)
  (params (Component :type Actor%20Component%20Object%20Reference) (bReset :type Boolean))
  (bind _bp_comp_gpt (Variables|Default|GetBP_Comp_GPT))
  (bind _sound_introduction (Variables|OpenAI|GetSound_Introduction))
  (if (not (Variables|OpenAI|GetIsSoundPlaying))
    (Variables|/Game/BP/NPC/BP_Comp_GPT.BP_Comp_GPT_C|SetIsCloseTask (Variables|Default|GetBP_Comp_GPT) false)
    (if (Default|CheckNetworking (Variables|Default|GetBP_Comp_GPT)) ; 网络判断，失败播放预制提示音：文三介绍
      (Default|CallOpenAIWaitAIVoice _bp_comp_gpt (Variables|/Game/BP/NPC/BP_Comp_GPT.BP_Comp_GPT_C|GetDefaultGreeting _bp_comp_gpt))
      (else
        (Utilities|SwitchbySpeechStatus
          (:false
            (Variables|OpenAI|SetIsSoundPlaying true)
            (Audio|PlaySound2D _sound_introduction 1.0 1.0 0.0 0 0 :!pinned true) ; 播放网络链接失败的本地语音-文三介绍
            (Utilities|FlowControl|Delay (Variables|/Script/Engine.SoundBase|GetDuration _sound_introduction))
            (Variables|OpenAI|SetIsSoundPlaying false)))))))

(event OnComponentDeactivated(AudioCapture)
  (params (Component :type Actor%20Component%20Object%20Reference))
  (bind _bp_comp_gpt (Variables|Default|GetBP_Comp_GPT))
  (Default|SetAIRecordandVoiceStatus _bp_comp_gpt false false)
  (Default|OnClearTask _bp_comp_gpt))

(event OnAudioEnvelopeValue(AudioCapture)
  (params (EnvelopeValue :type Float%20%28single-precision%29))
  (bind _sound_warning (Variables|OpenAI|GetSound_Warning))
  (if (> EnvelopeValue 0.02)
    (if (Default|CheckNetworking (Variables|Default|GetBP_Comp_GPT)) ; 网络判断，失败播放预制提示音：链接失败
      (Default|CallOpenAIRecordingVoice (Variables|Default|GetBP_Comp_GPT))
      (else
        (Utilities|SwitchbySpeechStatus
          (:false
            (if (not (Variables|OpenAI|GetIsSoundPlaying))
              (Variables|OpenAI|SetIsSoundPlaying true)
              (Audio|PlaySound2D _sound_warning 1.0 1.0 0.0 0 0 :!pinned true) ; 播放网络链接失败的本地语音-检查网络
              (Utilities|FlowControl|Delay (Variables|/Script/Engine.SoundBase|GetDuration _sound_warning))
              (Variables|OpenAI|SetIsSoundPlaying false))))))))

(event EDSendMessage(BP_Comp_GPT)
  (params (Message :type String))
  (bind _ui_chat (Variables|OpenAI|GetUI_Chat))
  (Utilities|IsValid _ui_chat
    (:Is%20Valid
      (Default|OnSetChatMessage _ui_chat Message))))

(event EDNetStatus(BP_Comp_GPT)
  (params (IsConnected :type Boolean))
  (bind _ui_net (Variables|OpenAI|GetUI_Net))
  (Utilities|IsValid _ui_net
    (:Is%20Valid
      (Default|OnSetNetStatus _ui_net IsConnected))))

(event EventBeginPlay
  (bind _widget (Variables|Default|GetWidget))
  (bind _returnvalue (UserInterface|GetWidget _widget))
  (Rendering|SetVisibility _widget false false)
  (Utilities|IsValid _returnvalue
    (:Is%20Valid
      (bind _asui_chat_item (Utilities|Casting|CastToUI_ChatItem _returnvalue))
      (Variables|OpenAI|SetUI_Chat _asui_chat_item)
      (bind _returnvalue_2 (UserInterface|CreateWidget "/Game/BP/NPC/UI_NetWorking.UI_NetWorking_C"))
      (bind _output_get (Variables|OpenAI|SetUI_Net _returnvalue_2))
      (UserInterface|Viewport|AddtoViewport _output_get 0))))

(fn ConstructionScript)