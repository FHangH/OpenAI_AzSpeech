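; NPC component that holds voice or text conversations with the player through ChatGPT and Azure Speech.
; Recorded speech becomes text, goes to ChatGPT behind a persona prompt, and the reply is broadcast and played as synthesized 2D audio.
; Recording and waiting flags gate new recordings.
; A three-second timer probes both services and reloads each NPC's keys, persona, model and voice from an INI file.
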(event Custom|CallOpenAI_TextChat
  (params (Role :type EHttpGPTChatRole%20Enum :default "User") (Content :type String))
  (bind _message (Utilities|CallOpenAI Role Content)
    (:Updated
      (Default|CallEDSendMessage (.Content (Utilities|Struct|BreakHttpGPTChatMessage _message))))
    (:Completed
      (CallFunction|CallOpenAIWaitAIVoice (.Content (Utilities|Struct|BreakHttpGPTChatMessage _message))))))

(event Custom|CallOpenAI_RecordingVoice
  (Utilities|CheckGPTandSpeechStatus
    (:true
      (bind (_asynctaskproxy _finalstring) (|SpeechtoTextDefaultOptions "Default" "Default" "None")
        (:then
          (Utilities|SetAIRecordStatus true false))
        (:RecognitionCompleted
          (Utilities|SetAIRecordStatus false true)
          (Utilities|CheckTaskIsClose
            (:真
              (Utilities|SetAIRecordStatus false false)
              (Variables|OpenAI|Check|SetIsCloseTask false))
            (:false
              (if (Utilities|Enum|NotEqual(Enum) _finalstring "")
                (bind _message (Utilities|CallOpenAI "User" _finalstring)
                  (:Updated
                    (Default|CallEDSendMessage (.Content (Utilities|Struct|BreakHttpGPTChatMessage _message))))
                  (:Completed
                    (CallFunction|CallOpenAIWaitAIVoice (.Content (Utilities|Struct|BreakHttpGPTChatMessage _message)))))
                (else
                  (Utilities|SetAIRecordStatus false false))))))
        (:RecognitionFailed
          (Utilities|SetAIRecordStatus false false)
          (CallFunction|CallOpenAIWaitAIVoice (Variables|OpenAI|Config|offine|GetRetryMessage))
          (Default|CallEDSendMessage (Variables|OpenAI|Config|offine|GetRetryMessage)))))))

(event Custom|CallOpenAI_WaitAIVoice
  (params (Text :type String))
  (Utilities|CheckTaskIsClose
    (:false
      (if (Utilities|Enum|NotEqual(Enum) Text "")
        (Utilities|IsValid (Variables|OpenAI|Data|GetAISoundCue)
          (:Is%20Valid
            (Variables|OpenAI|Data|SetAISoundCue 0))
          (:Is%20Not%20Valid
            _))
        (bind (_asynctaskproxy _generatedsound) (|TexttoSoundWaveDefaultOptions Text "Default" "Default")
          (:then
            (Utilities|SetAIRecordStatus false true))
          (:SynthesisCompleted
            (bind _output_get (Variables|OpenAI|Data|SetAISoundCue _generatedsound))
            (Utilities|IsValid _output_get
              (:Is%20Valid
                (Utilities|FlowControl|Sequence
                  (:then_0
                    (Audio|PlaySound2D (Variables|OpenAI|Data|GetAISoundCue) 1.0 1.0 0.0 0 0)
                    (Default|CallEDSendMessage Text))
                  (:then_1
                    (Utilities|FlowControl|Delay (- (Math|Conversions|ToFloat(Integer) (/ (Class|AzSpeechSynthesizerTaskBase|GetAudioDuration _asynctaskproxy) 1000)) 0.5))
                    (Utilities|SetAIRecordStatus false false)))))))))))

(event Custom|SetAIRecordAndVoiceStatus
  (params (IsRecording :type Boolean) (IsWaitingAIVoice :type Boolean))
  (Utilities|SetAIRecordStatus IsRecording IsWaitingAIVoice))

(event Custom|OnCheckNetStatus
  (Utilities|CheckNetStatus
    (:Connected
      (Default|CallEDNetStatus true))
    (:Failed
      (Default|CallEDNetStatus false)))
  (CallFunction|CheckGPTandSpeechConfig)
  (Utilities|InitAzSpeech)
  (Utilities|InitChatGPT))

(event Custom|CheckGPTAndSpeechConfig
  (bind _npc_id (Variables|OpenAI|Config|GetNPC_ID))
  (Utilities|InitChatGPTConfig _npc_id)
  (Utilities|InitAzSpeechConfig _npc_id))

(event Custom|OnClearTask
  (Variables|OpenAI|Check|SetIsCloseTask true)
  (Utilities|ClearTask (stale Custom|CallOpenAI_RecordingVoice _asynctaskproxy)))

(event EventEndPlay
  (params (EndPlayReason :type EEndPlayReason%20Enum :default "Destroyed"))
  (Utilities|Time|ClearandInvalidateTimerbyHandle (Variables|OpenAI|Check|GetNetTimer)))

(event EventBeginPlay
  (Utilities|FlowControl|Sequence
    (:then_0
      (CallFunction|CheckGPTandSpeechConfig)
      ;[0 0 0 0.7] 初始化 Azure和ChatGPT
      (Utilities|InitAzSpeech)
      (Utilities|InitChatGPT)
      (Utilities|Time|SetTimerbyEvent (EventDispatchers|CreateEvent :!event Custom|OnCheckNetStatus) 3.0 true :!pinned true) ; 循环检查网络状态
    )
    (:then_1
      (Utilities|SetAIRecordStatus false false))))

(fn CheckNetworking
  (return (and (Variables|OpenAI|Check|GetIsChatConnected) (Variables|OpenAI|Check|GetIsAzSpeechConnected))))

(fn CheckSpeechStatus
  (return (Variables|OpenAI|Recording|GetIsRecording) (Variables|OpenAI|Recording|GetIsWaitingAIVoice)))